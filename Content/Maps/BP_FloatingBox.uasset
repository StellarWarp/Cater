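; BP_FloatingBox is a level actor that links itself to trigger objects able to activate or deactivate it.
; On BeginPlay it adds itself to the Activates list of each ActivateTrigger entry and the Deactivates list of each DeactivateTrigger entry.
; The graphs shown hold no floating or activation response logic.
; A NotNull helper, unused here, tests an object's path name against "None".
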(event `self.ReceiveBeginPlay`
  (`|ExecutionSequence`
    (:`then_0`
      (for _array_element (`self.ActivateTrigger`)
        (`KismetArrayLibrary.Array_Add` (`/Game/Maps/BoxActivationTrigger.Activates` _array_element) self)))
    (:`then_1`
      (for _array_element_2 (`self.DeactivateTrigger`)
        (`KismetArrayLibrary.Array_Add` (`/Game/Maps/BoxActivationTrigger.Deactivates` _array_element_2) self)))))

(fn `UserConstructionScript`)